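; Lockable hinged door that Interact toggles by yawing SmDoor through a timeline, ignoring calls while moving.
; Interact makes Degree positive unless IsInverted is set and only prints "Locked" until PickupKeyItem clears the lock.
; ForceInteractDoor sets an explicit open or closed state on a second timeline, bypassing the lock.
; Two nested spheres swap outer and inner icons on both sides as the player approaches or leaves.
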(event `/Game/Agate/Blueprint/Interface/I_Interactable.Interact`
  (params (Character :type "/Game/FirstPerson/Blueprints/BP_FirstPersonCharacter Object Reference"))
  (bind _degree (`self.Degree`))
  (if (`self.IsInverted`)
    (set `self.Degree` _degree)
    (else
      (set `self.Degree` (`KismetMathLibrary.Abs` _degree))))
  (if (`self.IsLocked`)
    (`KismetSystemLibrary.PrintString` "Locked")
    (elif (not (`self.IsMoving`))
      (set `self.IsMoving` true)
      (bind _output_get (set `self.IsOpened` (not (`self.IsOpened`))))
      (if _output_get
        (bind (_direction _dooralpha) (`Timeline|TL_Doors` :!via `PlayFromStart` :!label _label)
          (:`Update`
            (`SceneComponent.K2_SetRelativeRotation` (`self.Sm_Door`) (`KismetMathLibrary.MakeRotator` 0.0 0.0 (`KismetMathLibrary.Lerp` 0.0 (`self.Degree`) _dooralpha)) false false))
          (:`Finished`
            (set `self.IsMoving` false)))
        (else
          (goto _label :!via `ReverseFromEnd`))))))

(event `self.InnerShpere.OnComponentBeginOverlap`
  (params (OverlappedComponent :type "PrimitiveComponent Object Reference") (OtherActor :type "Actor Object Reference") (OtherComp :type "PrimitiveComponent Object Reference") (OtherBodyIndex :type Integer) (bFromSweep :type Boolean) (SweepResult :type "HitResult Structure (by ref)"))
  (if (== OtherActor (`GameplayStatics.GetPlayerCharacter` 0))
    (`SceneComponent.SetVisibility` (`self.Inner Icon Side A`) true false)
    (`SceneComponent.SetVisibility` (`self.Inner Icon Side B`) true false)
    (`SceneComponent.SetVisibility` (`self.Outer Icon Side A`) false false)
    (`SceneComponent.SetVisibility` (`self.Outer Icon Side B`) false false)))

(event `self.InnerShpere.OnComponentEndOverlap`
  (params (OverlappedComponent :type "PrimitiveComponent Object Reference") (OtherActor :type "Actor Object Reference") (OtherComp :type "PrimitiveComponent Object Reference") (OtherBodyIndex :type Integer))
  (if (== (`GameplayStatics.GetPlayerCharacter` 0) OtherActor)
    (`SceneComponent.SetVisibility` (`self.Inner Icon Side A`) false false)
    (`SceneComponent.SetVisibility` (`self.Inner Icon Side B`) false false)
    (`SceneComponent.SetVisibility` (`self.Outer Icon Side A`) true false)
    (`SceneComponent.SetVisibility` (`self.Outer Icon Side B`) true false)))

(event `self.OuterSphere.OnComponentBeginOverlap`
  (params (OverlappedComponent :type "PrimitiveComponent Object Reference") (OtherActor :type "Actor Object Reference") (OtherComp :type "PrimitiveComponent Object Reference") (OtherBodyIndex :type Integer) (bFromSweep :type Boolean) (SweepResult :type "HitResult Structure (by ref)"))
  (if (== OtherActor (`GameplayStatics.GetPlayerCharacter` 0))
    (`SceneComponent.SetVisibility` (`self.Outer Icon Side A`) true false)
    (`SceneComponent.SetVisibility` (`self.Outer Icon Side B`) true false)))

(event `self.OuterSphere.OnComponentEndOverlap`
  (params (OverlappedComponent :type "PrimitiveComponent Object Reference") (OtherActor :type "Actor Object Reference") (OtherComp :type "PrimitiveComponent Object Reference") (OtherBodyIndex :type Integer))
  (if (== (`GameplayStatics.GetPlayerCharacter` 0) OtherActor)
    (`SceneComponent.SetVisibility` (`self.Outer Icon Side A`) false false)
    (`SceneComponent.SetVisibility` (`self.Outer Icon Side B`) false false)))

(event `/Game/Agate/Blueprint/Interface/I_Interactable.Pickup Key Item`
  (params (Doors :type "/Game/Agate/Blueprint/BP_Doors Object Reference"))
  (set `self.IsLocked` false))

(event `ForceInteractDoor`
  (params (IsOpening :type Boolean))
  (if (not (`self.IsMoving`))
    (set `self.IsMoving` true)
    (bind _output_get (set `self.IsOpened` IsOpening))
    (if _output_get
      (bind (_direction _dooralpha) (`Timeline|Timeline_0` :!via `PlayFromStart` :!label _label_2)
        (:`Update`
          (`SceneComponent.K2_SetRelativeRotation` (`self.Sm_Door`) (`KismetMathLibrary.MakeRotator` 0.0 0.0 (`KismetMathLibrary.Lerp` 0.0 (`self.Degree`) _dooralpha)) false false))
        (:`Finished`
          (set `self.IsMoving` false)))
      (else
        (goto _label_2 :!via `ReverseFromEnd`)))))

(fn `UserConstructionScript`)