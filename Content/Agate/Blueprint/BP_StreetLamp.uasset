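; BP_StreetLamp is a street lamp actor that can be switched on or off.
; The ToggleLamp event stores the IsOn state, sets the SpotLight intensity to LightIntensity or zero, and shows or hides the Sphere component to match.
; The construction script applies the same logic from the current IsOn value, while BeginPlay, overlap and Tick are unused.
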(event `Toggle Lamp`
  (params (IsOn :type Boolean))
  (bind _spotlight (`self.SpotLight`))
  (bind _output_get (set `self.IsOn` IsOn))
  (if _output_get
    (`LightComponent.SetIntensity` _spotlight (`self.LightIntensity`))
    (else
      (`LightComponent.SetIntensity` _spotlight 0.0)))
  (`SceneComponent.SetVisibility` (`self.Sphere`) _output_get false))

(fn `UserConstructionScript`
  (bind _ison (`self.IsOn`))
  (bind _spotlight (`self.SpotLight`))
  (if _ison
    (`LightComponent.SetIntensity` _spotlight (`self.LightIntensity`))
    (else
      (`LightComponent.SetIntensity` _spotlight 0.0)))
  (`SceneComponent.SetVisibility` (`self.Sphere`) _ison false))