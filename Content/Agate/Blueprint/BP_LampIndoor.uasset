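; BP_LampIndoor is an indoor lamp actor that can be switched on or off.
; The ToggleLamp event stores IsOn, sets the RectLight intensity to LightIntensity or zero, and shows or hides the Cylinder component to match.
; The construction script repeats the same logic, so the placed lamp reflects its IsOn and LightIntensity values without running the game.
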(event `Toggle Lamp`
  (params (IsOn :type Boolean))
  (bind _rectlight (`self.RectLight`))
  (bind _output_get (set `self.IsOn` IsOn))
  (if _output_get
    (`LightComponent.SetIntensity` _rectlight (`self.LightIntensity`))
    (else
      (`LightComponent.SetIntensity` _rectlight 0.0)))
  (`SceneComponent.SetVisibility` (`self.Cylinder`) _output_get false))

(fn `UserConstructionScript`
  (bind _ison (`self.IsOn`))
  (bind _rectlight (`self.RectLight`))
  (if _ison
    (`LightComponent.SetIntensity` _rectlight (`self.LightIntensity`))
    (else
      (`LightComponent.SetIntensity` _rectlight 0.0)))
  (`SceneComponent.SetVisibility` (`self.Cylinder`) _ison false))