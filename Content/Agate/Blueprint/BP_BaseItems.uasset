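; Base world item that shows proximity icons to the player and can be inspected when interacted with.
; Overlapping the outer sphere shows one icon, which swaps to another inside the inner sphere.
; If inspectable, Interact spawns a BP_InspectionItem far from the origin and passes it the mesh, item details, pickup flag and itself.
; Construction script applies sphere radii, mesh, scale, icon placement and a debug toggle for the inner icon.
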(event `self.InnerSphere.OnComponentBeginOverlap`
  (params (OverlappedComponent :type "PrimitiveComponent Object Reference") (OtherActor :type "Actor Object Reference") (OtherComp :type "PrimitiveComponent Object Reference") (OtherBodyIndex :type Integer) (bFromSweep :type Boolean) (SweepResult :type "HitResult Structure (by ref)"))
  (if (== OtherActor (`GameplayStatics.GetPlayerCharacter` 0))
    (`SceneComponent.SetVisibility` (`self.Inner Sphere Icon`) true false)
    (`SceneComponent.SetVisibility` (`self.Outer Sphere Icon`) false false)))

(event `self.InnerSphere.OnComponentEndOverlap`
  (params (OverlappedComponent :type "PrimitiveComponent Object Reference") (OtherActor :type "Actor Object Reference") (OtherComp :type "PrimitiveComponent Object Reference") (OtherBodyIndex :type Integer))
  (if (== (`GameplayStatics.GetPlayerCharacter` 0) OtherActor)
    (`SceneComponent.SetVisibility` (`self.Inner Sphere Icon`) false false)
    (`SceneComponent.SetVisibility` (`self.Outer Sphere Icon`) true false)))

(event `self.OuterSphere.OnComponentBeginOverlap`
  (params (OverlappedComponent :type "PrimitiveComponent Object Reference") (OtherActor :type "Actor Object Reference") (OtherComp :type "PrimitiveComponent Object Reference") (OtherBodyIndex :type Integer) (bFromSweep :type Boolean) (SweepResult :type "HitResult Structure (by ref)"))
  (if (== OtherActor (`GameplayStatics.GetPlayerCharacter` 0))
    (`SceneComponent.SetVisibility` (`self.Outer Sphere Icon`) true false)))

(event `self.OuterSphere.OnComponentEndOverlap`
  (params (OverlappedComponent :type "PrimitiveComponent Object Reference") (OtherActor :type "Actor Object Reference") (OtherComp :type "PrimitiveComponent Object Reference") (OtherBodyIndex :type Integer))
  (if (== (`GameplayStatics.GetPlayerCharacter` 0) OtherActor)
    (`SceneComponent.SetVisibility` (`self.Outer Sphere Icon`) false false)))

(event `/Game/Agate/Blueprint/Interface/I_Interactable.Interact`
  (params (Character :type "/Game/FirstPerson/Blueprints/BP_FirstPersonCharacter Object Reference"))
  (if (`self.Is Inspect Able`)
    (bind _returnvalue (`|SpawnActorFromClass` "/Game/Agate/Blueprint/BP_InspectionItem.BP_InspectionItem_C" (`KismetMathLibrary.MakeTransform` (1000000000000.0 0.0 0.0)) "Undefined" "MultiplyWithRoot" null null))
    (`/Game/Agate/Blueprint/BP_InspectionItem.Set Item Rotation` _returnvalue (`self.Inspect Item Rotation`))
    (`/Game/Agate/Blueprint/BP_InspectionItem.Set Item Scale` _returnvalue (`self.Inspect Item Scale`))
    (`/Game/Agate/Blueprint/Interface/I_Interactable.Inspect` _returnvalue Character (`StaticMeshComponent.StaticMesh` (`self.StaticMesh`)) (`self.Item Name`) (`self.Item Description`) self (`self.Is Pickup Able`) (`self.ItemType`))))

(fn `UserConstructionScript`
  (bind _staticmesh (`self.StaticMesh`))
  (bind _inner_sphere_icon (`self.Inner Sphere Icon`))
  (`|ExecutionSequence`
    (:`then_0`
      (`SphereComponent.SetSphereRadius` (`self.InnerSphere`) (`self.Inner Sphere Radius`) true)
      (`SphereComponent.SetSphereRadius` (`self.OuterSphere`) (`self.Outer Sphere Radius`) true))
    (:`then_1`
      (`StaticMeshComponent.SetStaticMesh` _staticmesh (`self.Mesh`))
      (`SceneComponent.K2_SetWorldTransform` _staticmesh (`KismetMathLibrary.MakeTransform` (`SceneComponent.K2_GetComponentLocation` _staticmesh) (`SceneComponent.K2_GetComponentRotation` _staticmesh) (`self.Mesh Scale`)) false false))
    (:`then_2`
      (`SceneComponent.K2_SetRelativeLocation` _inner_sphere_icon (`self.Icon Location`) false false)
      (`SceneComponent.K2_SetRelativeLocation` (`self.Outer Sphere Icon`) (`self.Icon Location`) false false)
      (`SceneComponent.SetVisibility` _inner_sphere_icon (`self.IsDebugging`) false))))